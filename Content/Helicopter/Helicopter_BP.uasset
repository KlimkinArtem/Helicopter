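; Pilotable helicopter that a player possesses on entering, riding attached at the pilot socket until exit restores control.
; Throttle sets a target rotor speed; the smoothed speed feeds a lift curve, which also scales pitch and banked-turn rates.
; Tick moves it by hand-rolled, swept motion from previous-frame velocity, gravity, up-vector lift and extra horizontal thrust when tilted.
; Rotors spin with current speed, swapping to blur meshes and capping visual spin above a threshold.
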(event `self.ReceiveBeginPlay`
  (`self.UpdatePrevVersion`))

(event `InputAction|EnterVehicle`
  (params (Key :type "Key Structure"))
  (:`Pressed`
    (`self.Exit`)))

(event `InputAxis|HeliThrottle`
  (params (AxisValue :type "Float (single-precision)"))
  (set `self.TargetBladeRotationSpeed` (`KismetMathLibrary.FClamp` (+ (* AxisValue (`GameplayStatics.GetWorldDeltaSeconds`) (`self.ThrottleUpSpeed`)) (`self.TargetBladeRotationSpeed`)) 0.0 (`self.MaxBladeRotationSpeed`))))

(event `self.ReceiveTick`
  (params (DeltaSeconds :type "Float (single-precision)"))
  (`self.Tick` DeltaSeconds)
  (`self.RotateBlades` DeltaSeconds))

(event `InputAxis|HeliTurn`
  (params (AxisValue :type "Float (single-precision)"))
  (bind (_returnvalue_roll _returnvalue_pitch _returnvalue_yaw) (`KismetMathLibrary.BreakRotator` (`self.K2_GetActorRotation`)))
  (bind _output_get (set `self.CurrentTurn` (`KismetMathLibrary.FInterpTo` (`self.CurrentTurn`) (* AxisValue (`self.GetTurnSpeed`)) (`GameplayStatics.GetWorldDeltaSeconds`) 2.0)))
  (`self.K2_AddActorWorldRotation` (`KismetMathLibrary.MakeRotator` 0.0 0.0 _output_get))
  (`self.K2_SetActorRotation` (`KismetMathLibrary.MakeRotator` (* _output_get 40.0) _returnvalue_pitch _returnvalue_yaw)))

(event `InputAxis|HeliPitch`
  (params (AxisValue :type "Float (single-precision)"))
  (bind (_returnvalue_roll _returnvalue_pitch) (`KismetMathLibrary.BreakRotator` (`self.K2_GetActorRotation`)))
  (bind _output_get (set `self.CurrentPitch` (`KismetMathLibrary.FInterpTo` (`self.CurrentPitch`) (* AxisValue (`self.GetTurnSpeed`)) (`GameplayStatics.GetWorldDeltaSeconds`) 2.0)))
  (if (`KismetMathLibrary.InRange_FloatFloat` (+ _output_get _returnvalue_pitch) -89.0 89.0)
    (`self.K2_AddActorLocalRotation` (`KismetMathLibrary.MakeRotator` 0.0 _output_get))))

(fn `Enter`
  (params (Player :type "/Game/ThirdPersonCPP/Blueprints/ThirdPersonCharacter Object Reference") (ExitDelegate :type "Delegate (by ref)"))
  (add `self.OnExited` ExitDelegate)
  (bind _output_get (set `self.Occupant` Player))
  (`Controller.Possess` (`self.GetController` _output_get) self)
  (`self.K2_AttachToActor` (`self.Occupant`) self "pilot_sit" "SnapToTarget" "SnapToTarget" "SnapToTarget" true))

(fn `Exit`
  (`self.K2_DetachFromActor` (`self.Occupant`) "KeepWorld" "KeepWorld" "KeepWorld")
  (`self.K2_SetActorLocation` (`self.Occupant`) (`SceneComponent.K2_GetComponentLocation` (`self.EnterBoxLeft`)) false false)
  (`Controller.Possess` (`self.GetController`) (`self.Occupant`))
  (`self.OnExited`))

(fn `GetCurrentLift`
  (returns (Lift :type "Float (double-precision)"))
  (return (`CurveFloat.GetFloatValue` (`self.LiftCurve`) (`self.CurrentBladeRotationSpeed`))))

(fn `GetTurnSpeed`
  (returns (ReturnValue :type "Float (double-precision)"))
  (return (* (`self.TurnSpeed`) (`KismetMathLibrary.MapRangeClamped` (`self.GetCurrentLift`) 0.0 400.0 0.0 1.0))))

(fn `RotateBlades`
  (params (DeltaSeconds :type "Float (double-precision)"))
  (bind _returnvalue (* (`self.BlurBladeSpeed`) (`local.DeltaSeconds`)))
  (bind _returnvalue_2 (* (`self.CurrentBladeRotationSpeed`) (`local.DeltaSeconds`)))
  (if (> (`self.CurrentBladeRotationSpeed`) (`self.BlurBladeSpeed`))
    (`StaticMeshComponent.SetStaticMesh` (`self.Blades`) "/Game/Helicopter/Mesh/main_rotor_blade_blur.main_rotor_blade_blur")
    (`StaticMeshComponent.SetStaticMesh` (`self.RearBlade`) "/Game/Helicopter/Mesh/tail_rotor_blade_blur.tail_rotor_blade_blur")
    (`SceneComponent.K2_AddRelativeRotation` (`self.Rotor`) (`KismetMathLibrary.MakeRotator` 0.0 0.0 _returnvalue) false false)
    (`SceneComponent.K2_AddLocalRotation` (`self.RearRotor`) (`KismetMathLibrary.MakeRotator` 0.0 (* _returnvalue 2.0)) false false)
    (else
      (`StaticMeshComponent.SetStaticMesh` (`self.Blades`) "/Game/Helicopter/Mesh/main_rotor_blade.main_rotor_blade")
      (`StaticMeshComponent.SetStaticMesh` (`self.RearBlade`) "/Game/Helicopter/Mesh/rear_rotor_blade.rear_rotor_blade")
      (`SceneComponent.K2_AddRelativeRotation` (`self.Rotor`) (`KismetMathLibrary.MakeRotator` 0.0 0.0 _returnvalue_2) false false)
      (`SceneComponent.K2_AddLocalRotation` (`self.RearRotor`) (`KismetMathLibrary.MakeRotator` 0.0 (* _returnvalue_2 2.0)) false false))))

(fn `Tick`
  (params (DeltaSeconds :type "Float (double-precision)"))
  (bind (_returnvalue_x _returnvalue_y) (`KismetMathLibrary.BreakVector` (`self.GetActorUpVector`)))
  (`|ExecutionSequence`
    (:`then_0`
      ;[1 1 1] Update blade rotation speed to match target
      (set `self.CurrentBladeRotationSpeed` (`KismetMathLibrary.FInterpTo` (`self.CurrentBladeRotationSpeed`) (`self.TargetBladeRotationSpeed`) (`local.DeltaSeconds`) 1.0)))
    (:`then_1`
      ;[1 1 1] Calculate velocity and aceleration
      (set `self.Velocity` (* (- (`self.K2_GetActorLocation`) (`self.PrevPosition`)) (`local.DeltaSeconds`)))
      (set `self.Acceleration` (* (- (`self.Velocity`) (`self.PrevVelocity`)) (`local.DeltaSeconds`))))
    (:`then_2`
      (`self.UpdatePrevVersion`))
    (:`then_3`
      ;[1 1 1] Apply gravity
      (set `self.Acceleration` (+ (`self.Acceleration`) (0.0 0.0 -981.0)))
      ;[1 1 1] Apply lift
      (set `self.Acceleration` (+ (`self.Acceleration`) (* (`self.GetActorUpVector`) (`self.GetCurrentLift`))))
      ;[1 1 1] Simulate forward acceleration
      (set `self.Acceleration` (+ (`self.Acceleration`) (* (`KismetMathLibrary.MakeVector` _returnvalue_x _returnvalue_y) (* (`self.GetCurrentLift`) 2.0)))))
    (:`then_4`
      ;[1 1 1] Move Helicopter
      (`self.K2_AddActorWorldOffset` (+ (`self.Velocity`) (* (`self.Acceleration`) (`local.DeltaSeconds`))) true))))

(fn `UpdatePrevVersion`
  (set `self.PrevPosition` (`self.K2_GetActorLocation`))
  (set `self.PrevVelocity` (`self.Velocity`))
  (set `self.PrevAcceleration` (0.0 0.0 0.0)))

(fn `UserConstructionScript`)