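; Helicopter Blueprint, apparently built on a C++ base class, that adds the player HUD and handles rotor blade visuals.
; On BeginPlay it creates the HUD widget and adds it to the viewport.
; Two events swap the main and tail rotor static meshes between blurred and normal versions to suggest spinning blades.
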(event `self.ReceiveBeginPlay`
  (bind _returnvalue (`|CreateWidget` "/Game/Helicopter/HUD.HUD_C"))
  (`UserWidget.AddToViewport` _returnvalue 0))

(event `SetBladeBlur`
  (`StaticMeshComponent.SetStaticMesh` (`self.Blades`) "/Game/Helicopter/Mesh/main_rotor_blade_blur.main_rotor_blade_blur")
  (`StaticMeshComponent.SetStaticMesh` (`self.RearBlade`) "/Game/Helicopter/Mesh/tail_rotor_blade_blur.tail_rotor_blade_blur"))

(event `SetBladeBlurNormal`
  (`StaticMeshComponent.SetStaticMesh` (`self.Blades`) "/Game/Helicopter/Mesh/main_rotor_blade.main_rotor_blade")
  (`StaticMeshComponent.SetStaticMesh` (`self.RearBlade`) "/Game/Helicopter/Mesh/rear_rotor_blade.rear_rotor_blade"))

(fn `UserConstructionScript`)